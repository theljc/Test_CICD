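; Audio visualizer example actor that scales a cube to the spectrum of the sound it plays.
; On BeginPlay it plays the sound and converts each playback-percent callback into seconds using the sound's duration.
; That time samples precomputed non-real-time Constant-Q data on channel 0.
; Every band value sets the same cube's scale in turn, so only the last band's value remains visible.
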(event `self.ReceiveBeginPlay`
  (bind _audio (`self.Audio`))
  (`AudioComponent.SetSound` (`self.Audio`) (`self.New Sound`))
  (set `self.Duration` (`SoundBase.Duration` (`self.New Sound`)))
  (add `AudioComponent.OnAudioPlaybackPercent` _audio (delegate `OnAudioPlaybackPercent_Event`))
  (`AudioComponent.Play` _audio 0.0))

(event `OnAudioPlaybackPercent_Event`
  (params (PlayingSoundWave :type "SoundWave Object Reference") (PlaybackPercent :type "Float (single-precision)"))
  (bind _output_get (set `self.PlayBackTime` (* PlaybackPercent (`self.Duration`))))
  (for _array_element (`ConstantQNRT.GetNormalizedChannelConstantQAtTime` (`self.Sound QNRT`) _output_get 0)
    (`SceneComponent.SetWorldScale3D` (`self.Cube`) (`KismetMathLibrary.Conv_DoubleToVector` (* _array_element 5.0)))))

(fn `UserConstructionScript`)