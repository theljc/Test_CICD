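; BP_NPC is an NPC Blueprint that highlights itself and shows its name when the cursor hovers over it.
; The Construction Script applies the Tint colour to the mesh materials, and BeginPlay passes NPCName to the WBP_NPCName widget.
; Capsule cursor-over events set or clear an overlay material on the mesh and toggle the name widget's visibility.
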(event `self.ReceiveBeginPlay`
  (bind _aswbp_npcname (cast `/Game/QuestExamples/Widget/WBP_NPCName` (`WidgetComponent.GetWidget` (`self.Widget`))))
  (`/Game/QuestExamples/Widget/WBP_NPCName.Set NPCName` _aswbp_npcname (`KismetTextLibrary.Conv_NameToText` (`self.NPCName`))))

(event `self.CapsuleComponent.OnBeginCursorOver`
  (params (TouchedComponent :type "PrimitiveComponent Object Reference"))
  (`MeshComponent.SetOverlayMaterial` (`self.Mesh`) "/Game/QuestExamples/Material/M_Overlay_Inst.M_Overlay_Inst")
  (`SceneComponent.SetVisibility` (`self.Widget`) true false))

(event `self.CapsuleComponent.OnEndCursorOver`
  (params (TouchedComponent :type "PrimitiveComponent Object Reference"))
  (`MeshComponent.SetOverlayMaterial` (`self.Mesh`) null)
  (`SceneComponent.SetVisibility` (`self.Widget`) false false))

(fn `UserConstructionScript`
  (`MeshComponent.SetVectorParameterValueOnMaterials` (`self.Mesh`) "Tint" (`self.Tint`)))