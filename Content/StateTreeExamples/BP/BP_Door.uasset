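; BP_Door is a StateTree example door actor whose open and close motion is shown by moving a text component.
; It starts its StateTree on BeginPlay and can send it a tagged event.
; Open and Close use timelines to lerp the text up or down from its current position.
; Wrapper functions trigger these and return the timeline length, and another displays a state value on the text.
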(event `self.ReceiveBeginPlay`
  (`BrainComponent.StartLogic` (`self.StateTree`)))

(event `Send Event To StateTree`
  (`StateTreeComponent.SendStateTreeEvent` (`self.StateTree`) (make `StateTreeEvent` (struct :`TagName` "Test.StateTree.Tag2"))))

(event `Open`
  (bind _text_location (`self.Text Location`))
  (set `self.Text Location` (`SceneComponent.K2_GetComponentLocation` (`self.TextRender`)))
  (bind (_direction _newtrack_0) (`Timeline|Open Door Timeline` :!via `PlayFromStart`)
    (:`Update`
      (`SceneComponent.K2_SetWorldLocation` (`self.TextRender`) (`KismetMathLibrary.VLerp` _text_location (+ _text_location (0.0 0.0 60.0)) _newtrack_0) false false))))

(event `Close`
  (bind _text_location (`self.Text Location`))
  (set `self.Text Location` (`SceneComponent.K2_GetComponentLocation` (`self.TextRender`)))
  (bind (_direction _newtrack_0) (`Timeline|Close Door  Timeline` :!via `PlayFromStart`)
    (:`Update`
      (`SceneComponent.K2_SetWorldLocation` (`self.TextRender`) (`KismetMathLibrary.VLerp` _text_location (+ _text_location (0.0 0.0 -60.0)) _newtrack_0) false false))))

(fn `Close Door`
  (returns (Delay :type "Float (double-precision)"))
  (`self.Close`)
  (return (`TimelineComponent.GetTimelineLength` (`self.Close Door  Timeline`))))

(fn `Open Door`
  (returns (Delay :type "Float (double-precision)"))
  (`self.Open`)
  (return (`TimelineComponent.GetTimelineLength` (`self.Open Door Timeline`))))

(fn `Set State Text`
  (params (Value :type "Text (by ref)"))
  (`TextRenderComponent.K2_SetText` (`self.TextRender`) (`|FormatText` "State:{0}" Value)))

(fn `UserConstructionScript`)