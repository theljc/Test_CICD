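; BP_Tutorial_P9 is a physics example Blueprint that previews the projectile path of one of its moving components.
; Every Tick it runs an advanced projectile path prediction with collision tracing from that component's world location and velocity, ignoring itself.
; It joins consecutive path points with red debug lines and moves a second component to the predicted hit location as an impact marker.
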(event `self.ReceiveBeginPlay`)

(event `self.ReceiveTick`
  (params (DeltaSeconds :type "Float (single-precision)"))
  (bind _2 (`self.2`))
  (bind _predictresult (`GameplayStatics.Blueprint_PredictProjectilePath_Advanced` (make `PredictProjectilePathParams` :`StartLocation` (`SceneComponent.K2_GetComponentLocation` _2) :`LaunchVelocity` (`SceneComponent.GetComponentVelocity` _2) :`bTraceWithCollision` true :`ProjectileRadius` 20.0 :`ActorsToIgnore` (`|MakeArray` self :!type "Actor Object Reference"))))
  (bind (_pathdata _lasttracedestination _hitresult) (break `PredictProjectilePathResult` _predictresult))
  (for (_array_element _array_index) _pathdata
    (if (== _array_index 0)
      (bind _location (break `PredictProjectilePathPointData` _array_element))
      (set `self.Last Location` _location)
      (else
        (`KismetSystemLibrary.DrawDebugLine` _location (`self.Last Location`) (struct :`R` 1.0 :`A` 1.0) 0.0 1.0)
        (set `self.Last Location` _location))))
  (`SceneComponent.K2_SetWorldLocation` (`self.3`) (`.Location` (`GameplayStatics.BreakHitResult` _hitresult)) false false))

(fn `UserConstructionScript`)