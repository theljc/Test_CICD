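; BP_Tutorial_P5 is a physics tutorial Blueprint that applies timed radial forces to an actor built from twenty procedurally added cubes.
; The construction script adds each mesh to CubeArray and creates a physics constraint with that mesh as its first component.
; After a delay on BeginPlay, a radial force component spawns at a random cube's relative location.
; After another delay, it is destroyed and replaced by one at the root's relative location.
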(event `self.ReceiveBeginPlay`
  (`KismetSystemLibrary.Delay` 2.0)
  (bind _returnvalue (`AddComponent|NODE_AddRadialForceComponent-0` :`bManualAttachment` true :`RelativeTransform` (`KismetMathLibrary.MakeTransform` (`SceneComponent.RelativeLocation` (`KismetArrayLibrary.Array_Random` (`self.Cube Array`))))))
  (`KismetSystemLibrary.Delay` 2.0)
  (`ActorComponent.K2_DestroyComponent` _returnvalue)
  (`AddComponent|NODE_AddRadialForceComponent-1` :`bManualAttachment` true :`RelativeTransform` (`KismetMathLibrary.MakeTransform` (`SceneComponent.RelativeLocation` (`self.DefaultSceneRoot`)))))

(fn `UserConstructionScript`
  (for _ (range 20)
    (bind _returnvalue (`AddComponent|NODE_AddStaticMeshComponent-0`))
    (`KismetArrayLibrary.Array_AddUnique` (`self.Cube Array`) _returnvalue)
    (bind _returnvalue_2 (`AddComponent|NODE_AddPhysicsConstraintComponent-0`))
    (`PhysicsConstraintComponent.SetConstrainedComponents` _returnvalue_2 _returnvalue "None" null "None")))