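; BP_Tutorial_P6_2 is a tutorial actor that moves its Cube component through waypoints marked by Arrow components.
; On BeginPlay it gathers all Arrow components into an array and starts a looping two-second timer.
; Each tick of the timer calls MoveComponentTo toward the current arrow's relative location, then advances the index, wrapping to zero after the last arrow for an endless loop.
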(event `self.ReceiveBeginPlay`
  (set `self.Arrow Array` (`self.K2_GetComponentsByClass` "/Script/Engine.ArrowComponent"))
  (`KismetSystemLibrary.K2_SetTimerDelegate` (delegate `CustomEvent`) 2.0 true))

(event `CustomEvent`
  (`KismetSystemLibrary.MoveComponentTo` (`self.Cube`) (`SceneComponent.RelativeLocation` (`|GetArrayItem` (`self.Arrow Array`) (`self.Index`))))
  (if (== (mod (+ (`self.Index`) 1) (`KismetArrayLibrary.Array_Length` (`self.Arrow Array`))) 0)
    (set `self.Index` 0)
    (else
      (`/Engine/EditorBlueprintResources/StandardMacros.IncrementInt` (`self.Index`)))))

(fn `UserConstructionScript`)