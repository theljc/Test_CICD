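; BP_Cable is a physics-example cable actor meant to link a Left and a Right object.
; Its construction script snaps a valid Left to the Cable component's first socket, keeping relative scale.
; The Right branch only checks validity, and the event graph is empty.
; Unconnected nodes that would move the actor to Left, then stretch and aim it at Right, never run.
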(fn `UserConstructionScript`
  (`|ExecutionSequence`
    (:`then_0`
      (bind _left (`self.Left`)
        (:`then`
          (`self.K2_AttachToComponent` _left (`self.Cable`) (`|GetArrayItem` (`SceneComponent.GetAllSocketNames` (`self.Cable`))) "SnapToTarget" "SnapToTarget" "KeepRelative" true))
        (:`else`)))
    (:`then_1`
      (bind _right (`self.Right`)
        (:`then`)
        (:`else`)))))