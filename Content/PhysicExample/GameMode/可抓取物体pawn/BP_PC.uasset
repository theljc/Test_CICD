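; BP_PC is a player controller that lets the player paint or erase on a render target with the mouse, and exposes Inventory and Quest components.
; While left mouse is held with CanDraw set, Tick traces the surface under the cursor and feeds its collision UV to a dynamic brush material drawn into the target.
; Shift at press selects erasing, and C clears the target.
; Drawing suspends the default input mapping; release restores it and the saved control rotation.
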(event `self.ReceiveBeginPlay`
  (bind _returnvalue (subsystem `EnhancedInputLocalPlayerSubsystem`))
  (`/Engine/EditorBlueprintResources/StandardMacros.IsValid` _returnvalue
    (:`Is Valid`
      (`EnhancedInputSubsystemInterface.AddMappingContext` _returnvalue (`self.Default Mapping Context`) 0 (struct))
      (bind _returnvalue_2 (`KismetMaterialLibrary.CreateDynamicMaterialInstance` "/Game/MaterialExample/RenderTarget/M_Brush.M_Brush"))
      (set `self.DMI_Brush` _returnvalue_2))))

(event `self.ReceiveTick`
  (params (DeltaSeconds :type "Float (single-precision)"))
  (bind (_bblockinghit _binitialoverlap _time _distance _location _impactpoint _normal) (`GameplayStatics.BreakHitResult` (`self.GetHitResultUnderCursorByChannel` "TraceTypeQuery1")))
  (`|ExecutionSequence`
    (:`then_0`
      (if (`self.StartDraw`)
        (bind _outhit (`KismetSystemLibrary.LineTraceSingle` (+ _location _normal) (- _location _normal) "TraceTypeQuery1" true))
        (bind (_x _y) (`KismetMathLibrary.BreakVector2D` (`GameplayStatics.FindCollisionUV` _outhit)))
        (`MaterialInstanceDynamic.SetVectorParameterValue` (`self.DMI_Brush`) "DrawPosition" (`KismetMathLibrary.MakeColor` _x _y 0.0 0.0))
        (if (`self.Erase`)
          (`MaterialInstanceDynamic.SetScalarParameterValue` (`self.DMI_Brush`) "Erase" 0.0)
          (else
            (`MaterialInstanceDynamic.SetScalarParameterValue` (`self.DMI_Brush`) "Erase" 1.0)))
        (`KismetRenderingLibrary.DrawMaterialToRenderTarget` (`self.Render Target`) (`self.DMI_Brush`))))))

(event `Key|LeftMouseButton`
  (params (Key :type "Key Structure"))
  (:`Pressed`
    (if (`self.CanDraw`)
      (set `self.Erase` (`KismetInputLibrary.ModifierKeysState_IsShiftDown` (`KismetInputLibrary.GetModifierKeysState`)))
      (set `self.Control Rotation` (`self.GetControlRotation`))
      (set `self.Controlled Pawn` (`self.K2_GetPawn`))
      (set `self.StartDraw` true)
      (`EnhancedInputSubsystemInterface.RemoveMappingContext` (subsystem `EnhancedInputLocalPlayerSubsystem`) (`self.Default Mapping Context`) (struct))))
  (:`Released`
    (if (`self.CanDraw`)
      (bind _controlled_pawn (`self.Controlled Pawn`)
        (:`then`
          (`self.SetControlRotation` (`self.Control Rotation`))
          (set `self.StartDraw` false)
          (`EnhancedInputSubsystemInterface.AddMappingContext` (subsystem `EnhancedInputLocalPlayerSubsystem`) (`self.Default Mapping Context`) 0 (struct)))
        (:`else`)))))

(event `Key|C`
  (params (Key :type "Key Structure"))
  (:`Pressed`
    (`KismetRenderingLibrary.ClearRenderTarget2D` (`self.Render Target`))))

(fn `GetInventoryComponent`
  (returns (ReturnValue :type "InventoryComponent Object Reference"))
  (return (`self.Inventory`)))

(fn `GetQuestComponent`
  (returns (ReturnValue :type "QuestComponent Object Reference"))
  (return (`self.Quest`)))

(fn `UserConstructionScript`)