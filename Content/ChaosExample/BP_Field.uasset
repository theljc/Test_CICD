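; BP_Field is a Chaos physics field actor that creates a delayed explosion to break destructible geometry.
; Shortly after BeginPlay it spawns a Niagara explosion at its location, then applies an external cluster strain field with linear radial falloff.
; A sphere component sets the field's center and radius.
; A radial linear velocity field is also built in the graph but is unconnected, so it never runs.
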(event `self.ReceiveBeginPlay`
  (bind _sphere (`self.Sphere`))
  (`KismetSystemLibrary.Delay` 1.5)
  (`|ExecutionSequence`
    (:`then_0`
      (`NiagaraFunctionLibrary.SpawnSystemAtLocation` "/Game/NiagaraExplosion01/Niagaras/Air/N_ExplosionAir_004.N_ExplosionAir_004" (`self.K2_GetActorLocation`)))
    (:`then_1`
      (`FieldSystemComponent.ApplyPhysicsField` (`self.FieldSystem`) true "Field_ExternalClusterStrain" null (`RadialFalloff.SetRadialFalloff` (`self.RadialFalloff`) 100.0 0.0 1.0 0.0 (`SphereComponent.GetScaledSphereRadius` _sphere) (`SceneComponent.K2_GetComponentLocation` _sphere) "Field_Falloff_Linear")))))

(fn `UserConstructionScript`)