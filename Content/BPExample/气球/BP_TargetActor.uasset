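; BP_TargetActor is a Cube that gathers attached balloons until it rises fast enough.
; A looping timer spawns a BP_Ballon at a random horizontal offset above the Cube, stores it in Ballons and calls its Connect to link it to the Cube.
; Tick watches the Cube's vertical velocity and clears the spawn timer once upward speed passes a threshold with balloons present.
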(event `self.ReceiveBeginPlay`
  (bind _returnvalue (`KismetSystemLibrary.K2_SetTimerDelegate` (delegate `Spawn`) 2.0 true))
  (set `self.TimerHandle` _returnvalue))

(event `Spawn`
  (bind _returnvalue (`KismetMathLibrary.RandomFloatInRange` -50.0 50.0))
  (bind _returnvalue_2 (`|SpawnActorFromClass` "/Game/BPExample/气球/BP_Ballon.BP_Ballon_C" (`KismetMathLibrary.MakeTransform` (+ (`SceneComponent.K2_GetComponentLocation` (`self.Cube`)) (`KismetMathLibrary.MakeVector` _returnvalue _returnvalue 100.0))) "Undefined" "MultiplyWithRoot" null null))
  (`KismetArrayLibrary.Array_AddUnique` (`self.Ballons`) _returnvalue_2)
  (`/Game/BPExample/气球/BP_Ballon.Connect` _returnvalue_2 (`self.Cube`) (`SceneComponent.K2_GetComponentLocation` (`self.Cube`)) "root"))

(event `self.ReceiveTick`
  (params (DeltaSeconds :type "Float (single-precision)"))
  (bind _timerhandle (`self.TimerHandle`))
  (bind (_returnvalue_x _returnvalue_y _returnvalue_z) (`KismetMathLibrary.BreakVector` (`SceneComponent.GetComponentVelocity` (`self.Cube`))))
  (if (and (> _returnvalue_z 100.0) (`KismetArrayLibrary.Array_IsNotEmpty` (`self.Ballons`)))
    (if (`KismetSystemLibrary.K2_IsValidTimerHandle` _timerhandle)
      (`KismetSystemLibrary.K2_ClearAndInvalidateTimerHandle` _timerhandle))))

(fn `UserConstructionScript`)