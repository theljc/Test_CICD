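; BP_Ballon is a physics balloon actor that can be tethered to another component.
; Every tick it applies a constant upward force to its Sphere to create lift.
; The Connect event links a given component and bone to the Sphere through a PhysicsConstraint.
; It also attaches the Cable end to that component, converting the world attach location into the component's local space.
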(event `self.ReceiveBeginPlay`)

(event `self.ReceiveTick`
  (params (DeltaSeconds :type "Float (single-precision)"))
  (`PrimitiveComponent.AddForce` (`self.Sphere`) (0.0 0.0 20000.0) "None" false))

(event `Connect`
  (params (Component :type "PrimitiveComponent Object Reference") (AttachLocation :type "Vector Structure") (BoneName :type Name))
  (bind _cable (`self.Cable`))
  (`PhysicsConstraintComponent.SetConstrainedComponents` (`self.PhysicsConstraint`) Component BoneName (`self.Sphere`) "None")
  (`CableComponent.SetAttachEndToComponent` _cable Component "None")
  (set `CableComponent.EndLocation` (`KismetMathLibrary.InverseTransformLocation` (`SceneComponent.K2_GetComponentToWorld` Component) AttachLocation) _cable))

(fn `UserConstructionScript`)