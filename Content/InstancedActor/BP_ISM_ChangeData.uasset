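; BP_ISM_ChangeData fills per-instance custom data with random 0–1 values on every InstancedStaticMeshComponent of a referenced InstancedActor.
; UpdateInstancedMeshData reseeds a random stream for repeatable results, then passes each component to SetCustomData.
; SetCustomData loops over instance indices writing three data slots, though only the first write receives the loop index.
; Each iteration adds and removes a temporary instance to force a data refresh.
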(event `Update Instanced Mesh  Data`
  (bind _instancedactor (`self.InstancedActor`)
    (:`then`
      (`KismetMathLibrary.SetRandomStreamSeed` (`self.Random Stream`) (`self.Seed`))
      (for _array_element (`self.K2_GetComponentsByClass` _instancedactor "/Script/Engine.InstancedStaticMeshComponent")
        (`self.Set Custom Data` _array_element)))
    (:`else`)))

(fn `Set Custom Data`
  (params (`Instanced Mesh Component` :type "InstancedStaticMeshComponent Object Reference"))
  (bind _returnvalue (`KismetMathLibrary.RandomFloatInRangeFromStream` (`self.Random Stream`) 0.0 1.0))
  (for _index (range (+ (`InstancedStaticMeshComponent.GetInstanceCount` `Instanced Mesh Component`) 1))
    (`InstancedStaticMeshComponent.SetCustomDataValue` `Instanced Mesh Component` _index 0 _returnvalue false)
    (`InstancedStaticMeshComponent.SetCustomDataValue` `Instanced Mesh Component` 0 1 _returnvalue false)
    (`InstancedStaticMeshComponent.SetCustomDataValue` `Instanced Mesh Component` 0 2 _returnvalue false)
    ; 刷新数据
    (bind _returnvalue_2 (`InstancedStaticMeshComponent.AddInstance` `Instanced Mesh Component` (`KismetMathLibrary.MakeTransform` (0.0 0.0 0.0)) true))
    (`InstancedStaticMeshComponent.RemoveInstance` `Instanced Mesh Component` _returnvalue_2)))

(fn `UserConstructionScript`)