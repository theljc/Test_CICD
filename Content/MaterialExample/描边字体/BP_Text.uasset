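; BP_Text is a material-example actor that displays configurable outlined text through a TextRender component.
; Its construction script sets the text, then creates a dynamic material instance from the component's first material.
; It passes the actor's color, brightness and outline thickness variables into that instance as material parameters.
; The event graph holds only disabled placeholder events, so nothing runs at play time or per tick.
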(fn `UserConstructionScript`
  (bind _textrender (`self.TextRender`))
  (`TextRenderComponent.K2_SetText` (`self.TextRender`) (`self.Text`))
  (bind _returnvalue (`PrimitiveComponent.CreateDynamicMaterialInstance` _textrender 0 (`PrimitiveComponent.GetMaterial` _textrender 0) "None"))
  (`MaterialInstanceDynamic.SetVectorParameterValue` _returnvalue "Color" (`self.Color`))
  (`MaterialInstanceDynamic.SetScalarParameterValue` _returnvalue "Brightness" (`self.Brightness`))
  (`MaterialInstanceDynamic.SetScalarParameterValue` _returnvalue "Outline Tickness" (`self.Outline Tickness`)))