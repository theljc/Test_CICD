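; BP_ChangeMaterial is a material example actor that animates a looping dissolve on its Sphere component.
; BeginPlay starts a timeline whose track blends the "Dissolve" scalar parameter between -1 and 1 on the sphere's materials.
; When the timeline finishes, it pauses briefly and plays in the opposite direction, producing an endless ping-pong effect.
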(event `self.ReceiveBeginPlay`
  (`TimelineComponent.PlayFromStart` (`self.Timeline`)))

(fn `UserConstructionScript`)