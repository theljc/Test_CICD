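; BP_CombustionActor is a material-example actor that supplies the position and size of a burn effect area to materials through the MPC_Burn parameter collection.
; SetMPCParam writes the Sphere component's world location and scale into the collection's Location and Scale vector parameters.
; It runs from the Construction Script and BeginPlay with no per-tick update, so the values refresh on construction and at game start.
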(event `self.ReceiveBeginPlay`
  (`self.Set MPC Param`))

(fn `Set MPC Param`
  (`KismetMaterialLibrary.SetVectorParameterValue` "/Game/MaterialExample/烧毁效果/MPC_Burn.MPC_Burn" "Location" (`KismetMathLibrary.Conv_VectorToLinearColor` (`SceneComponent.K2_GetComponentLocation` (`self.Sphere`))))
  (`KismetMaterialLibrary.SetVectorParameterValue` "/Game/MaterialExample/烧毁效果/MPC_Burn.MPC_Burn" "Scale" (`KismetMathLibrary.Conv_VectorToLinearColor` (`SceneComponent.K2_GetComponentScale` (`self.Sphere`)))))

(fn `UserConstructionScript`
  (`self.Set MPC Param`))