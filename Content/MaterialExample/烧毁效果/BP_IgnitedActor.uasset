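; BP_IgnitedActor is a material example actor that plays a burn effect on its static mesh, then removes itself.
; The construction script creates a dynamic instance of M_Burn_Inst on the mesh's first material slot.
; Tick raises the BoundsScale parameter by a fixed, frame-rate-dependent step until it reaches a limit, then destroys the actor.
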(event `self.ReceiveTick`
  (params (DeltaSeconds :type "Float (single-precision)"))
  (if (< (`self.ScaleValue`) 8000.0)
    (bind _output_get (set `self.ScaleValue` (+ (`self.ScaleValue`) 8.0)))
    (`MaterialInstanceDynamic.SetScalarParameterValue` (`self.DMI_Mesh`) "BoundsScale" _output_get)
    (else
      (`self.K2_DestroyActor`))))

(fn `UserConstructionScript`
  (bind _returnvalue (`PrimitiveComponent.CreateDynamicMaterialInstance` (`self.StaticMeshComponent`) 0 "/Game/MaterialExample/烧毁效果/M_Burn_Inst.M_Burn_Inst" "None"))
  (set `self.DMI_Mesh` _returnvalue))