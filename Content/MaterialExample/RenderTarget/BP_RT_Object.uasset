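; BP_RT_Object is a render target example actor whose Box trigger switches drawing on for the player standing inside it.
; On begin overlap by the player's controlled pawn, it casts the player controller to BP_PC, enables CanDraw and shows the mouse cursor.
; End overlap clears both flags, leaving the drawing itself outside this Blueprint.
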(event `self.ReceiveBeginPlay`)

(event `self.Box.OnComponentBeginOverlap`
  (params (OverlappedComponent :type "PrimitiveComponent Object Reference") (OtherActor :type "Actor Object Reference") (OtherComp :type "PrimitiveComponent Object Reference") (OtherBodyIndex :type Integer) (bFromSweep :type Boolean) (SweepResult :type "HitResult Structure (by ref)"))
  (if (== OtherActor (`Controller.K2_GetPawn` (`GameplayStatics.GetPlayerController` 0)))
    (bind _asbp_pc (cast `/Game/PhysicExample/GameMode/可抓取物体pawn/BP_PC` (`GameplayStatics.GetPlayerController` 0)))
    (set `/Game/PhysicExample/GameMode/可抓取物体pawn/BP_PC.CanDraw` true _asbp_pc)
    (set `PlayerController.bShowMouseCursor` true _asbp_pc)))

(event `self.Box.OnComponentEndOverlap`
  (params (OverlappedComponent :type "PrimitiveComponent Object Reference") (OtherActor :type "Actor Object Reference") (OtherComp :type "PrimitiveComponent Object Reference") (OtherBodyIndex :type Integer))
  (if (== OtherActor (`Controller.K2_GetPawn` (`GameplayStatics.GetPlayerController` 0)))
    (bind _asbp_pc (cast `/Game/PhysicExample/GameMode/可抓取物体pawn/BP_PC` (`GameplayStatics.GetPlayerController` 0)))
    (set `/Game/PhysicExample/GameMode/可抓取物体pawn/BP_PC.CanDraw` false _asbp_pc)
    (set `PlayerController.bShowMouseCursor` false _asbp_pc)))

(fn `UserConstructionScript`)