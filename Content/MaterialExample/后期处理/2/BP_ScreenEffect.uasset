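; Trigger-area actor that plays a recurring post-process screen effect while the player's pawn is inside its Box.
; Construction adds a dynamic instance of M_PostProcess_2_Inst to the PostProcess settings.
; Box overlaps pause and unpause a looping timer, sized from both timelines plus Duration and a one-second gap.
; Each tick of that timer randomizes Direction, animates MinStep through Appear, waits Duration, then fades Opacity through Fade.
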(event `self.ReceiveBeginPlay`
  (bind _returnvalue (`KismetSystemLibrary.K2_SetTimerDelegate` (delegate `Show Effect`) (+ (`TimelineComponent.GetScaledTimelineLength` (`self.Fade`)) (`TimelineComponent.GetScaledTimelineLength` (`self.Appear`)) (`self.Duration`) 1.0) true))
  (bind _output_get (set `self.TimerHandle` _returnvalue))
  (`KismetSystemLibrary.K2_PauseTimerHandle` _output_get))

(event `Show Effect`
  (`MaterialInstanceDynamic.SetScalarParameterValue` (`self.DMI_PostProcess`) "MinStep" 1.5)
  (`MaterialInstanceDynamic.SetScalarParameterValue` (`self.DMI_PostProcess`) "Opacity" 1.0)
  (`MaterialInstanceDynamic.SetScalarParameterValue` (`self.DMI_PostProcess`) "Direction" (`KismetMathLibrary.RandomFloatInRange` 0.0 1.0))
  (`TimelineComponent.PlayFromStart` (`self.Appear`)))

(event `self.Box.OnComponentBeginOverlap`
  (params (OverlappedComponent :type "PrimitiveComponent Object Reference") (OtherActor :type "Actor Object Reference") (OtherComp :type "PrimitiveComponent Object Reference") (OtherBodyIndex :type Integer) (bFromSweep :type Boolean) (SweepResult :type "HitResult Structure (by ref)"))
  (if (and (== OtherActor (`Controller.K2_GetPawn` (`GameplayStatics.GetPlayerController` 0))) (`KismetSystemLibrary.K2_IsValidTimerHandle` (`self.TimerHandle`)))
    (`KismetSystemLibrary.K2_UnPauseTimerHandle` (`self.TimerHandle`))))

(event `self.Box.OnComponentEndOverlap`
  (params (OverlappedComponent :type "PrimitiveComponent Object Reference") (OtherActor :type "Actor Object Reference") (OtherComp :type "PrimitiveComponent Object Reference") (OtherBodyIndex :type Integer))
  (if (and (== OtherActor (`Controller.K2_GetPawn` (`GameplayStatics.GetPlayerController` 0))) (`KismetSystemLibrary.K2_IsValidTimerHandle` (`self.TimerHandle`)))
    (`KismetSystemLibrary.K2_PauseTimerHandle` (`self.TimerHandle`))))

(fn `UserConstructionScript`
  (bind _returnvalue (`KismetMaterialLibrary.CreateDynamicMaterialInstance` "/Game/MaterialExample/后期处理/2/M_PostProcess_2_Inst.M_PostProcess_2_Inst"))
  (set `self.DMI_PostProcess` _returnvalue)
  (set `PostProcessComponent.Settings` (make `PostProcessSettings` :`WeightedBlendables` (make `WeightedBlendables` (`|MakeArray` (make `WeightedBlendable` 1.0 (`self.DMI_PostProcess`))))) (`self.PostProcess`)))